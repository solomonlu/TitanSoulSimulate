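; BP_Arrow is the player's retrievable projectile arrow, shot with strength-scaled speed and gravity.
; SetHoming pulls it back toward the player without gravity, passing through static world geometry.
; A hit fires OnHit, then after a short delay enables the pickup sphere, whose player overlap calls BP_Hero's PickupArrow.
; Mutual move-ignore prevents player collisions, and re-setting the updated component on stop keeps the projectile movement reusable.
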(event OnProjectileStop(ProjectileMovement)
  (params (ImpactResult :type Hit%20Result%20Structure%20%28by%20ref%29))
  ;[1 1 1] https://answers.unrealengine.com/questions/84836/projectile-movement-disables-velocity-changes-afte.html
  (Components|Movement|SetUpdatedComponent (Variables|Default|GetProjectileMovement) (Variables|Default|GetArrowCollsion)))

(event OnComponentBeginOverlap(Sphere)
  (params (OverlappedComponent :type Primitive%20Component%20Object%20Reference) (OtherActor :type Actor%20Object%20Reference) (OtherComp :type Primitive%20Component%20Object%20Reference) (OtherBodyIndex :type Integer) (bFromSweep :type Boolean) (SweepResult :type Hit%20Result%20Structure%20%28by%20ref%29))
  (Development|PrintString (Utilities|GetDisplayName OtherActor))
  (if (== OtherActor (Game|GetPlayerCharacter 0))
    (Components|Activation|Deactivate (Variables|Default|GetProjectileMovement))
    (Collision|SetCollisionEnabled (Variables|Default|GetSphere) "NoCollision")
    (CallFunction|SetIgnorePlayer true)
    (Default|PickupArrow (.AsBP%20Hero (Utilities|Casting|CastToBP_Hero (Game|GetPlayerCharacter 0))))))

(event OnComponentHit(ArrowCollsion)
  (params (HitComponent :type Primitive%20Component%20Object%20Reference) (OtherActor :type Actor%20Object%20Reference) (OtherComp :type Primitive%20Component%20Object%20Reference) (NormalImpulse :type Vector :default "0, 0, 0") (Hit :type Hit%20Result%20Structure%20%28by%20ref%29))
  (Development|PrintString (Utilities|String|Append (Utilities|GetDisplayName OtherActor) "." (Utilities|GetObjectName OtherComp)))
  (Default|CallOnHit)
  (Utilities|FlowControl|Delay 0.5) ; 如果离墙壁特别近射箭，会出现奇怪的现象，所以延迟一会
  (Collision|SetCollisionProfileName (Variables|Default|GetSphere) "OverlapOnlyPawn" :!class /Script/Engine.PrimitiveComponent)
  (Collision|SetCollisionEnabled (Variables|Default|GetSphere) "QueryAndPhysics")
  (CallFunction|SetIgnorePlayer false))

(event Custom|Shoot
  (params (ShootDirection :type Vector) (ShootStrength :type Float%20%28single-precision%29))
  (Utilities|FlowControl|Sequence
    (:then_0
      (CallFunction|SetIgnorePlayer true)
      (Collision|SetCollisionResponsetoChannel (Variables|Default|GetArrowCollsion) "ECC_WorldStatic" "ECR_Block"))
    (:then_1
      (Components|Activation|Activate (Variables|Default|GetProjectileMovement) true)
      (Variables|/Script/Engine.MovementComponent|SetVelocity (Variables|Default|GetProjectileMovement) (* ShootDirection (Math|Float|Lerp 1.2e+03 3.5e+03 (/ ShootStrength 1e+02))))
      (Variables|/Script/Engine.ProjectileMovementComponent|SetProjectileGravityScale (Variables|Default|GetProjectileMovement) 1.0))))

(event Custom|SetHoming
  (Variables|/Script/Engine.ProjectileMovementComponent|SetbIsHomingProjectile (Variables|Default|GetProjectileMovement) true)
  (Variables|/Script/Engine.ProjectileMovementComponent|SetHomingTargetComponent (Variables|Default|GetProjectileMovement) (Variables|/Script/Engine.Character|GetCapsuleComponent (Game|GetPlayerCharacter 0)))
  (Variables|/Script/Engine.ProjectileMovementComponent|SetHomingAccelerationMagnitude (Variables|Default|GetProjectileMovement) 1.5e+03)
  (Variables|/Script/Engine.ProjectileMovementComponent|SetProjectileGravityScale (Variables|Default|GetProjectileMovement) 0.0)
  (Components|Activation|Activate (Variables|Default|GetProjectileMovement) true)
  (Collision|SetCollisionResponsetoChannel (Variables|Default|GetArrowCollsion) "ECC_WorldStatic" "ECR_Ignore"))

(event EventBeginPlay
  (Utilities|FlowControl|Delay 0.5)
  (CallFunction|SetIgnorePlayer true))

(fn ConstructionScript)

(fn SetIgnorePlayer
  (params (ShouldIgnore :type Boolean))
  (Collision|IgnoreActorwhenMoving (Variables|Default|GetArrowCollsion) (Game|GetPlayerCharacter 0) ShouldIgnore)
  (Collision|IgnoreActorwhenMoving (Variables|/Script/Engine.Character|GetCapsuleComponent (Game|GetPlayerCharacter 0)) self ShouldIgnore))