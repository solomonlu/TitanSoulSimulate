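; Greater Spider boss that repeatedly chases the player and performs melee attacks.
; Its skill loop starts when the anim instance signals spawn end and continues while the boss is not dead.
; The random skill choice currently always resolves to melee: face the player, approach with AIMoveTo, then play one of three random attack montages.
; Montage completion leads to a short delay before the next decision.
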(event Custom|CastMeleeAttack
  (Transformation|SetActorRotation (Math|Rotator|FindLookatRotation (Transformation|GetActorLocation) (Transformation|GetActorLocation (Game|GetPlayerCharacter 0))))
  (AI|AIMoveTo (.AsAIController (Utilities|Casting|CastToAIController (Pawn|GetController))) "0, 0, 0" (Game|GetPlayerCharacter 0) 5e+02 "Disable" "Default" true true
    (:OnMoveFinished
      (Animation|Montage|PlayMontage (Variables|Character|GetMesh) (Utilities|Select :Index (Math|Random|RandomIntegerinRange 0 2) :Option%200 "/Game/TitanSoulSimulate/SkeletalMesh/Spider/Animation/ExoGame_Greater_Spider_Attack_Melee_Montage.ExoGame_Greater_Spider_Attack_Melee_Montage" :Option%201 "/Game/TitanSoulSimulate/SkeletalMesh/Spider/Animation/ExoGame_Greater_Spider_Attack_Melee_B_Montage.ExoGame_Greater_Spider_Attack_Melee_B_Montage" :Option%202 "/Game/TitanSoulSimulate/SkeletalMesh/Spider/Animation/ExoGame_Greater_Spider_Attack_Melee_C_Montage.ExoGame_Greater_Spider_Attack_Melee_C_Montage")
        (:OnCompleted
          (Utilities|FlowControl|Delay 1.0)
          (CallFunction|DesideWhatSkill))))))

(event Custom|OnSpawnEnd_Event
  (CallFunction|DesideWhatSkill))

(event Custom|DesideWhatSkill
  (if (not (Variables|Default|GetIsDeath))
    (switch int (Math|Random|RandomIntegerinRange 0 2)
      (:0
        _)
      (:1
        _)
      (:2
        _))
    (CallFunction|CastMeleeAttack)))

(event EventBeginPlay
  (EventDispatchers|AssignOnSpawnEnd (.AsBPA%20Greater%20Spider (Utilities|Casting|CastToBPA_GreaterSpider (Components|SkeletalMesh|GetAnimInstance (Variables|Character|GetMesh)))) (delegate Custom|OnSpawnEnd_Event)))

(fn ConstructionScript)