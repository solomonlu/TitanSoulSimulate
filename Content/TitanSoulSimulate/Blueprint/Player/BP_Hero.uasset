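; Player hero character for a bow game with one reusable arrow that it shoots, absorbs and picks up.
; Pull-interface input sets aim rotation and pulling state, while BPA_Hero animation delegates drive charging, walk speed and arrow release.
; Tick builds or decays pull strength, shown through a progress material, and faces the arrow while absorbing.
; Any damage triggers a one-time ragdoll death and game-over widget; Revive is empty.
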(event Custom|AbsorbArrow
  ;[1 1 1] Absorb Arrow
  (Variables|/Game/ModularRPGHeroesPolyart/Meshes/BPA_Hero.BPA_Hero_C|SetIsAbsorbing (.AsBPA%20Hero (Utilities|Casting|CastToBPA_Hero (Components|SkeletalMesh|GetAnimInstance (Variables|Character|GetMesh)))) true)
  (CallFunction|AimStart)
  (Variables|/Script/Engine.CharacterMovementComponent|SetMaxWalkSpeed (Variables|Character|GetCharacterMovement) 0.0))

(event Custom|Roll
  ;[1 1 1] Roll
  (Animation|Montage|PlayMontage (Variables|Character|GetMesh) "/Game/ModularRPGHeroesPolyart/Animations/BowStance/Roll_Bow_RMAnim_Montage.Roll_Bow_RMAnim_Montage" 1.5))

(event Custom|OnDeath
  (bind _capsulecomponent (Variables|Collision|GetCapsuleComponent))
  (bind _mesh (Variables|Character|GetMesh))
  ;[1 1 1] Damage And Death
  (Input|DisableInput (.AsPlayer%20Controller (Utilities|Casting|CastToPlayerController (Pawn|GetController))))
  (Animation|Montage|MontageStop (Components|SkeletalMesh|GetAnimInstance (Variables|Character|GetMesh)) 0.0 0)
  (Collision|SetCollisionResponsetoAllChannels _capsulecomponent "ECR_Ignore")
  (Collision|SetCollisionResponsetoChannel _capsulecomponent "ECC_WorldStatic" "ECR_Block")
  (Collision|SetCollisionProfileName _mesh "Ragdoll" :!class /Script/Engine.PrimitiveComponent)
  (Physics|SetSimulatePhysics _mesh true)
  ;;[1 1 1] Show Game Over Widget
  (Utilities|FlowControl|Delay 2.8)
  (bind _returnvalue (UserInterface|CreateWidget "/Game/TitanSoulSimulate/UMG/Gameplay/UMG_GameOver.UMG_GameOver_C" (.AsPlayer%20Controller (Utilities|Casting|CastToPlayerController (Pawn|GetController)))))
  (UserInterface|Viewport|AddtoViewport _returnvalue 0))

(event Custom|AimEnd
  ;[1 1 1] Pull Bow Function
  (Variables|/Script/Engine.CharacterMovementComponent|SetbUseControllerDesiredRotation (Variables|Character|GetCharacterMovement) false)
  (Variables|/Script/Engine.CharacterMovementComponent|SetbOrientRotationToMovement (Variables|Character|GetCharacterMovement) true))

(event Custom|PickupArrow
  ;[1 1 1] Pickup Arrow
  (Transformation|SetActorTransform (Variables|Default|GetMyArrow) (Math|Transform|MakeTransform "-64.000000, 0, 0" "0,180.000000, 0" "1,1,1"))
  (Transformation|AttachComponentToComponent (Variables|Default|GetMyArrow) (Variables|Character|GetMesh) "hand_rSocket" "KeepRelative" "KeepRelative" "KeepWorld" false)
  (Variables|/Game/ModularRPGHeroesPolyart/Meshes/BPA_Hero.BPA_Hero_C|SethasArrow (.AsBPA%20Hero (Utilities|Casting|CastToBPA_Hero (Components|SkeletalMesh|GetAnimInstance (Variables|Character|GetMesh)))) true)
  (Variables|/Game/ModularRPGHeroesPolyart/Meshes/BPA_Hero.BPA_Hero_C|SetIsAbsorbing (.AsBPA%20Hero (Utilities|Casting|CastToBPA_Hero (Components|SkeletalMesh|GetAnimInstance (Variables|Character|GetMesh)))) false)
  (CallFunction|AimEnd)
  (Variables|/Script/Engine.CharacterMovementComponent|SetMaxWalkSpeed (Variables|Character|GetCharacterMovement) 4e+02)
  (Default|CallOnPickupArrow))

(event Custom|Revive
  ;[1 1 1] Damage And Death
)

(event Custom|AimStart
  ;[1 1 1] Pull Bow Function
  (Variables|/Script/Engine.CharacterMovementComponent|SetbUseControllerDesiredRotation (Variables|Character|GetCharacterMovement) true)
  (Variables|/Script/Engine.CharacterMovementComponent|SetbOrientRotationToMovement (Variables|Character|GetCharacterMovement) false))

(event EventBeginPlay
  (bind _returnvalue (Game|GetPlayerController 0))
  ;[1 1 1] begin play
  (Utilities|FlowControl|Sequence
    (:then_0
      (Utilities|FlowControl|Delay 0.1)
      (Class|PlayerController|ActivateTouchInterface _returnvalue "/Game/TopDownBP/Character/LeftVirtualJoystickOnly.LeftVirtualJoystickOnly")
      (bind _returnvalue_2 (UserInterface|CreateWidget "/Game/TitanSoulSimulate/UMG/Gameplay/UMG_GameMainWidget.UMG_GameMainWidget_C" _returnvalue))
      (UserInterface|Viewport|AddtoViewport _returnvalue_2 0))
    (:then_1
      (|AnimEventBind))
    (:then_4
      (bind _returnvalue_3 (Game|SpawnActorfromClass "/Game/TitanSoulSimulate/Blueprint/BP_Arrow.BP_Arrow_C" (Math|Transform|MakeTransform "-64.000000, 0, 0" "0,180.000000, 0" "1,1,1") "Undefined" 0 0))
      (bind _output_get (Variables|Default|SetMyArrow _returnvalue_3))
      (Transformation|AttachComponentToComponent _output_get (Variables|Character|GetMesh) "hand_rSocket" "KeepRelative" "KeepRelative" "KeepWorld" false))))

(event EventDestroyed
  (Actor|DestroyActor (Variables|Default|GetMyArrow)))

(event EventTick
  (params (DeltaSeconds :type Float%20%28single-precision%29))
  (Utilities|FlowControl|Sequence
    (:then_1
      ;[1 1 1] Poll Strength
      (Variables|Default|SetPullingStrength (Math|Float|Clamp(Float) (+ (Variables|Default|GetPullingStrength) (select (Variables|Default|GetIsStoragingPower) (* DeltaSeconds (Variables|Default|GetPullingStrengthIncreaseFactor)) (* DeltaSeconds -1.0 (Variables|Default|GetPullingStrengthDecreaseFactor)))) 0.0 1e+02)))
    (:then_2
      ;[1 1 1] absorb rotation
      (if (Variables|/Game/ModularRPGHeroesPolyart/Meshes/BPA_Hero.BPA_Hero_C|GetIsAbsorbing (.AsBPA%20Hero (Utilities|Casting|CastToBPA_Hero (Components|SkeletalMesh|GetAnimInstance (Variables|Character|GetMesh)))))
        (Pawn|SetControlRotation (Pawn|GetController) (Math|Rotator|MakeRotator 0.0 0.0 (.yaw (Math|Rotator|FindLookatRotation (Transformation|GetActorLocation) (Transformation|GetActorLocation (Variables|Default|GetMyArrow))))))))))

(event EventOnPullStart
  ;[1 1 1] Pull Bow Interface
  (CallFunction|AimStart))

(event Game|Damage|EventAnyDamage
  (params (Damage :type Float%20%28single-precision%29) (DamageType :type Damage%20Type%20Object%20Reference) (InstigatedBy :type Controller%20Object%20Reference) (DamageCauser :type Actor%20Object%20Reference))
  ;[1 1 1] Damage And Death
  (Utilities|FlowControl|DoOnce false
    (:Completed
      (CallFunction|OnDeath))))

(event EventOnPullTick
  (params (PullStartVector :type Vector :default "0, 0, 0") (PullTargetVector :type Vector :default "0, 0, 0"))
  ;[1 1 1] Pull Bow Interface
  (|PullTick PullStartVector PullTargetVector))

(event EventOnPullEnd
  ;[1 1 1] Pull Bow Interface
  (Variables|Default|SetIsPullingBow false)
  (if (<= (Variables|Default|GetPullingStrength) 0.0) ; 为解决玩家还未发生pull就松手的情况，这里判断一下
    (CallFunction|AimEnd)))

(event Input|AxisEvents|InputAxisMoveForward
  (params (AxisValue :type Float%20%28single-precision%29))
  ;[1 1 1] Movement
  (Class|PawnMovementComponent|AddInputVector (Variables|Character|GetCharacterMovement) (* "1.000000, 0, 0" AxisValue) false))

(event Input|AxisEvents|InputAxisMoveRight
  (params (AxisValue :type Float%20%28single-precision%29))
  ;[1 1 1] Movement
  (Class|PawnMovementComponent|AddInputVector (Variables|Character|GetCharacterMovement) (* "0,1.000000, 0" AxisValue) false))

(fn ConstructionScript
  (bind _returnvalue (Rendering|Material|CreateDynamicMaterialInstance (Variables|Default|GetPullStrengthProgress) 0 "/Game/RoboBars/Materials/ExamplesSurface/MI_DivisionSmooth.MI_DivisionSmooth" "None" :!class /Script/Engine.PrimitiveComponent))
  (bind _output_get (Variables|Default|SetPullStrengthMaterial _returnvalue))
  (Rendering|Material|SetScalarParameterValue _output_get "Progress" 0.0 :!class /Script/Engine.MaterialInstanceDynamic))

(fn OnRepIsPullingBow
  (Variables|/Game/ModularRPGHeroesPolyart/Meshes/BPA_Hero.BPA_Hero_C|SetIsPullingBow (.AsBPA%20Hero (Utilities|Casting|CastToBPA_Hero (Components|SkeletalMesh|GetAnimInstance (Variables|Character|GetMesh)))) (Variables|Default|GetIsPullingBow)))

(fn OnRepPullingStrength
  (if (> (Variables|Default|GetPullingStrength) 0.0)
    (Development|SetHiddeninGame (Variables|Default|GetPullStrengthProgress) false false)
    (Rendering|Material|SetScalarParameterValue (Variables|Default|GetPullStrengthMaterial) "Progress" (/ (Variables|Default|GetPullingStrength) 1e+02) :!class /Script/Engine.MaterialInstanceDynamic)
    (else
      (Development|SetHiddeninGame (Variables|Default|GetPullStrengthProgress) true false))))

(event Custom|OnAimEnd_Event
  (CallFunction|AimEnd))

(event Custom|OnShootEnd_Event
  (if (not (Variables|Default|GetIsPullingBow))
    (CallFunction|AimEnd)
    (Variables|/Game/ModularRPGHeroesPolyart/Meshes/BPA_Hero.BPA_Hero_C|SethasArrow (.AsBPA%20Hero (Utilities|Casting|CastToBPA_Hero (Components|SkeletalMesh|GetAnimInstance (Variables|Character|GetMesh)))) false)))

(event Custom|OnShootStart_Event
  (Transformation|DetachFromActor (Variables|Default|GetMyArrow) "KeepWorld" "KeepWorld" "KeepWorld")
  (Default|Shoot (Variables|Default|GetMyArrow) (Math|Rotator|GetRotationXVector (Pawn|GetControlRotation :!class /Script/Engine.Pawn)) (Variables|Default|GetShootStrength))
  (Default|CallOnShootArrow (Variables|Default|GetMyArrow)))

(event Custom|OnPollingStart_Event
  (CallFunction|AimStart)
  (Variables|Default|SetIsStoragingPower true)
  (Variables|/Script/Engine.CharacterMovementComponent|SetMaxWalkSpeed (Variables|Character|GetCharacterMovement) 2e+02))

(event Custom|OnPollingEnd_Event
  (CallFunction|AimEnd)
  (Variables|Default|SetIsStoragingPower false)
  (Variables|/Script/Engine.CharacterMovementComponent|SetMaxWalkSpeed (Variables|Character|GetCharacterMovement) 4e+02)
  (Variables|Default|SetShootStrength (Variables|Default|GetPullingStrength)))